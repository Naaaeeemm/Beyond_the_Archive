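; BP_FrameManager is a puzzle manager that watches four frame stands and activates a target frame once all are solved.
; On BeginPlay it leaves FrameToReveal visible but disables its collision.
; Tick polls IsSolved on every stand and, through a DoOnce, unhides the frame and enables its collision a single time.
; Despite the reveal naming, only collision effectively changes, since the frame is never hidden here.
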(event `self.ReceiveBeginPlay`
  (bind _frametoreveal (`self.FrameToReveal`))
  (`self.SetActorHiddenInGame` _frametoreveal false)
  (`self.SetActorEnableCollision` _frametoreveal false))

(event `self.ReceiveTick`
  (params (DeltaSeconds :type "Float (single-precision)"))
  (bind _frametoreveal (`self.FrameToReveal`))
  (if (and (`/Game/Blueprints/FrameArrange/BP_FrameStand.IsSolved?` (`self.FrameStand`)) (`/Game/Blueprints/FrameArrange/BP_FrameStand.IsSolved?` (`self.FrameStand_1`)) (`/Game/Blueprints/FrameArrange/BP_FrameStand.IsSolved?` (`self.FrameStand_2`)) (`/Game/Blueprints/FrameArrange/BP_FrameStand.IsSolved?` (`self.FrameStand_3`)))
    (`/Engine/EditorBlueprintResources/StandardMacros.DoOnce` false
      (:`Completed`
        (`self.SetActorHiddenInGame` _frametoreveal false)
        (`self.SetActorEnableCollision` _frametoreveal true)))))

(fn `UserConstructionScript`)