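; Game instance that owns the player's settings save and applies saved audio volumes at startup.
; Init loads the "Settings" slot or creates a new BP_SettingsSave, then retries each tick until a game mode is valid.
; It then pushes BYDMix with master, music and effects sound class overrides.
; Shutdown writes the object back to the slot, and ReturnSettingSave exposes it to other code.
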(event `self.ReceiveInit`
  (bind _returnvalue (`GameplayStatics.DoesSaveGameExist` "Settings"))
  (if _returnvalue
    (bind _returnvalue_2 (`GameplayStatics.LoadGameFromSlot` "Settings"))
    (bind _asbp_settings_save (cast `/Game/Blueprints/Save/BP_SettingsSave` _returnvalue_2))
    (set `self.SettingsSave` _asbp_settings_save)
    (else
      (bind _returnvalue_3 (`GameplayStatics.CreateSaveGameObject` "/Game/Blueprints/Save/BP_SettingsSave.BP_SettingsSave_C"))
      (set `self.SettingsSave` _returnvalue_3)))
  (`/Engine/EditorBlueprintResources/StandardMacros.IsValid` (`GameplayStatics.GetGameMode`) :!label _label
    (:`Is Valid`
      (`GameplayStatics.SetSoundMixClassOverride` "/Game/Audio/BYDMix.BYDMix" "/Game/Audio/BYDMaster.BYDMaster" (`/Game/Blueprints/Save/BP_SettingsSave.MasterVolume` (`self.SettingsSave`)) 1.0 0.0)
      (`GameplayStatics.SetSoundMixClassOverride` "/Game/Audio/BYDMix.BYDMix" "/Game/Audio/BYDMusic.BYDMusic" (`/Game/Blueprints/Save/BP_SettingsSave.MusicVolume` (`self.SettingsSave`)) 1.0 0.0)
      (`GameplayStatics.SetSoundMixClassOverride` "/Game/Audio/BYDMix.BYDMix" "/Game/Audio/BYDSFX.BYDSFX" (`/Game/Blueprints/Save/BP_SettingsSave.EffectsVolume` (`self.SettingsSave`)) 1.0 0.0)
      (`GameplayStatics.PushSoundMixModifier` "/Game/Audio/BYDMix.BYDMix"))
    (:`Is Not Valid`
      (`KismetSystemLibrary.DelayUntilNextTick`)
      (goto _label))))

(event `self.ReceiveShutdown`
  (`GameplayStatics.SaveGameToSlot` (`self.SettingsSave`) "Settings"))

(fn `Return Setting Save`
  (returns (SettingSaveRef :type "/Game/Blueprints/Save/BP_SettingsSave Object Reference"))
  (return (`self.SettingsSave`)))