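; Possessable Flow-style puzzle where the player links same-colored key nodes on a 5x5 cube grid.
; An assigned FrameStand or Numpad keeps it locked until solved; interacting then shows a tutorial widget.
; Selecting a key node sets the active color, which cursor moves paint onto empty cubes until reaching its match, with colored cubes blocking.
; Connecting every key node fires the solved event, disables re-entry and returns to the character; exiting early resets the board.
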(event `OnSolved_Event`
  (set `self.CanBePossessed` true))

(event `self.ReceiveBeginPlay`
  ; Setup
  (`parent.ReceiveBeginPlay`)
  (set `self.Cube` (`|MakeArray` (`self.Cube 1x1`) (`self.Cube 1x2`) (`self.Cube 1x3`) (`self.Cube 1x4`) (`self.Cube 1x5`) (`self.Cube 2x1`) (`self.Cube 2x2`) (`self.Cube 2x3`) (`self.Cube 2x4`) (`self.Cube 2x5`) (`self.Cube 3x1`) (`self.Cube 3x2`) (`self.Cube 3x3`) (`self.Cube 3x4`) (`self.Cube 3x5`) (`self.Cube 4x1`) (`self.Cube 4x2`) (`self.Cube 4x3`) (`self.Cube 4x4`) (`self.Cube 4x5`) (`self.Cube 5x1`) (`self.Cube 5x2`) (`self.Cube 5x3`) (`self.Cube 5x4`) (`self.Cube 5x5`)))
  (`|ExecutionSequence`
    (:`then_0`
      (`/Engine/EditorBlueprintResources/StandardMacros.IsValid` (`self.FrameStand`)
        (:`Is Valid`
          (set `self.CanBePossessed` false)
          (add `/Game/Blueprints/FrameArrange/BP_FrameStand.OnSolved` (`self.FrameStand`) (delegate `OnSolved_Event`)))))
    (:`then_1`
      (`/Engine/EditorBlueprintResources/StandardMacros.IsValid` (`self.Numpad`)
        (:`Is Valid`
          (set `self.CanBePossessed` false)
          (add `/Game/Blueprints/Numpad/BP_KeypadPawn.PuzzleSolve` (`self.Numpad`) (delegate `Numpad_Solved`)))))))

(event `Numpad_Solved`
  (set `self.CanBePossessed` true))

(event `/Game/Blueprints/InteractionInterface.Interact`
  (params (PlayerCharacter :type "/Game/Blueprints/Character/BP_FirstPersonCharacter Object Reference"))
  ; Possess & UnPossess
  (if (`self.CanBePossessed`)
    (`parent.Interact` PlayerCharacter)
    (`self.UpdateHighlightOfSelectedCube` true)
    (`KismetSystemLibrary.Delay` 0.5)
    (bind _returnvalue (`|CreateWidget` "/Game/UI/BPW/BPW_ColorConnectTut.BPW_ColorConnectTut_C" (`GameplayStatics.GetPlayerController` 0)))
    (bind _output_get (set `self.ColorConnectWidget` _returnvalue))
    (`UserWidget.AddToPlayerScreen` _output_get 0)))

(event `self.Return to Character`
  ; Possess & UnPossess
  (`Widget.RemoveFromParent` (`self.ColorConnectWidget`))
  (`self.UpdateHighlightOfSelectedCube` false)
  (`parent.Return to Character`))

(event `EnhancedInput|/Game/Input/Actions/IA_Interact`
  (params (ActionValue :type Boolean) (ElapsedSeconds :type "Float (double-precision)") (TriggeredSeconds :type "Float (double-precision)") (InputAction :type "InputAction Object Reference" :default "/Game/Input/Actions/IA_Interact.IA_Interact"))
  ;[0.15 0.03555 0.04451 0.5] Inputs
  (:`Triggered`
    (`self.TrySelectNode`)
    (`GameplayStatics.PlaySound2D` "/Game/Audio/SFX/ColorConnectInteract.ColorConnectInteract" 1.0 1.0 0.0 null null)))

(event `EnhancedInput|/Game/Input/Actions/IA_Puzzle/IA_NavigateUp`
  (params (ActionValue :type Boolean) (ElapsedSeconds :type "Float (double-precision)") (TriggeredSeconds :type "Float (double-precision)") (InputAction :type "InputAction Object Reference" :default "/Game/Input/Actions/IA_Puzzle/IA_NavigateUp.IA_NavigateUp"))
  ; Navigation
  (:`Triggered`
    (`self.NavigateCubes` -5)
    (`GameplayStatics.PlaySound2D` "/Game/Audio/SFX/ColorConnectMove.ColorConnectMove" 1.0 1.0 0.0 null null :!label _label)))

(event `EnhancedInput|/Game/Input/Actions/IA_Puzzle/IA_NavigateDown`
  (params (ActionValue :type Boolean) (ElapsedSeconds :type "Float (double-precision)") (TriggeredSeconds :type "Float (double-precision)") (InputAction :type "InputAction Object Reference" :default "/Game/Input/Actions/IA_Puzzle/IA_NavigateDown.IA_NavigateDown"))
  ; Navigation
  (:`Triggered`
    (`self.NavigateCubes` 5)
    (goto _label)))

(event `EnhancedInput|/Game/Input/Actions/IA_Puzzle/IA_Reset`
  (params (ActionValue :type Boolean) (ElapsedSeconds :type "Float (double-precision)") (TriggeredSeconds :type "Float (double-precision)") (InputAction :type "InputAction Object Reference" :default "/Game/Input/Actions/IA_Puzzle/IA_Reset.IA_Reset"))
  ;[0.15 0.03555 0.04451 0.5] Inputs
  (:`Triggered`
    (`self.Reset`)))

(event `EnhancedInput|/Game/Input/Actions/IA_Puzzle/IA_NavigateRight`
  (params (ActionValue :type Boolean) (ElapsedSeconds :type "Float (double-precision)") (TriggeredSeconds :type "Float (double-precision)") (InputAction :type "InputAction Object Reference" :default "/Game/Input/Actions/IA_Puzzle/IA_NavigateRight.IA_NavigateRight"))
  ; Navigation
  (:`Triggered`
    (`self.NavigateCubes` 1)
    (goto _label)))

(event `EnhancedInput|/Game/Input/Actions/IA_Puzzle/IA_ExitPuzzle`
  (params (ActionValue :type Boolean) (ElapsedSeconds :type "Float (double-precision)") (TriggeredSeconds :type "Float (double-precision)") (InputAction :type "InputAction Object Reference" :default "/Game/Input/Actions/IA_Puzzle/IA_ExitPuzzle.IA_ExitPuzzle"))
  ;[0.15 0.03555 0.04451 0.5] Inputs
  (:`Triggered`
    (`self.Reset`)
    (`self.Return to Character`)))

(event `EnhancedInput|/Game/Input/Actions/IA_Puzzle/IA_NavigateLeft`
  (params (ActionValue :type Boolean) (ElapsedSeconds :type "Float (double-precision)") (TriggeredSeconds :type "Float (double-precision)") (InputAction :type "InputAction Object Reference" :default "/Game/Input/Actions/IA_Puzzle/IA_NavigateLeft.IA_NavigateLeft"))
  ; Navigation
  (:`Triggered`
    (`self.NavigateCubes` -1)
    (goto _label)))

(fn `ConnectKeyNodes`
  (`|ExecutionSequence`
    (:`then_0`
      ; Mark all Nodes of selected Color as connected
      (set `/Game/Blueprints/ColorConnect/BP_ColorPuzzleComponent.IsConnected` true (`self.GetSelectedColor`))
      (for _array_element (`self.Cube`)
        (if (`|EnumEquality` (`/Game/Blueprints/ColorConnect/BP_ColorPuzzleComponent.PuzzleColor` _array_element) (`self.CurrentColor`))
          (set `/Game/Blueprints/ColorConnect/BP_ColorPuzzleComponent.IsConnected` true _array_element))))
    (:`then_1`
      ; After Connected turn current color white
      (set `self.CurrentColor` "NewEnumerator0")
      (set `self.SelectedKeyNode` null)
      (`KismetSystemLibrary.PrintString` "deselected/connected"))
    (:`then_2`
      ; Event after Puzzle is completed
      (if (`self.IsPuzzleComplete`)
        (`GameplayStatics.PlaySound2D` "/Game/Audio/SFX/ColorConnectFinished.ColorConnectFinished" 1.0 1.0 0.0 null null)
        (`self.SolvePuzzle`)
        (`self.Return to Character`)))))

(fn `GetSelectedColor`
  (returns (Output :type "/Game/Blueprints/ColorConnect/BP_ColorPuzzleComponent Object Reference"))
  (return (`|GetArrayItem` (`self.Cube`) (`self.CurrentCubeIndex`))))

(fn `IsBottomRow`
  (params (CubeIndex :type Integer))
  (returns (ReturnValue :type Boolean))
  (return (>= CubeIndex 20)))

(fn `IsLeftMostColumn`
  (params (CubeIndex :type Integer))
  (returns (ReturnValue :type Boolean))
  (return (or (== CubeIndex 0) (== CubeIndex 5) (== CubeIndex 10) (== CubeIndex 15) (== CubeIndex 20))))

(fn `IsPuzzleComplete`
  (returns (Result :type Boolean))
  ; If all Colors Connected
  (for _array_element (`self.Cube`)
    (if (`/Game/Blueprints/ColorConnect/BP_ColorPuzzleComponent.IsKeyNode` _array_element)
      (if (not (`/Game/Blueprints/ColorConnect/BP_ColorPuzzleComponent.IsConnected` _array_element))
        ;;[0.15 0.007031 0.007031 0.5] CheckFalseOrItWontDoSomething
        (return false))))
  ;;[0.15 0.01328 0.01328 0.5] Completed to check if ALL are connected
  (return true))

(fn `IsRightMostColumn`
  (params (CubeIndex :type Integer))
  (returns (ReturnValue :type Boolean))
  (return (or (== CubeIndex 4) (== CubeIndex 9) (== CubeIndex 14) (== CubeIndex 19) (== CubeIndex 24) (== CubeIndex 25))))

(fn `IsTopRow`
  (params (CubeIndex :type Integer))
  (returns (ReturnValue :type Boolean))
  (return (<= CubeIndex 4)))

(fn `NavigateCubes`
  (params (Direction :type Integer))
  (if (not (or (and (`self.IsTopRow` (`self.CurrentCubeIndex`)) (== (`local.Direction`) -5)) (and (`self.IsBottomRow` (`self.CurrentCubeIndex`)) (== (`local.Direction`) 5)) (and (`self.IsRightMostColumn` (`self.CurrentCubeIndex`)) (== (`local.Direction`) 1)) (and (`self.IsLeftMostColumn` (`self.CurrentCubeIndex`)) (== (`local.Direction`) -1))))
    (`self.UpdateHighlightOfSelectedCube` false)
    (set `self.CurrentCubeIndex` (+ (`self.CurrentCubeIndex`) Direction))
    (`|ExecutionSequence`
      (:`then_0`
        (if (> (`self.CurrentCubeIndex`) (`KismetArrayLibrary.Array_LastIndex` (`self.Cube`)))
          (set `self.CurrentCubeIndex` (- (`self.CurrentCubeIndex`) (`KismetArrayLibrary.Array_Length` (`self.Cube`))))))
      (:`then_1`
        (if (< (`self.CurrentCubeIndex`) 0)
          (set `self.CurrentCubeIndex` (+ (`self.CurrentCubeIndex`) (`KismetArrayLibrary.Array_Length` (`self.Cube`))))))
      (:`then_2`
        (bind _returnvalue (`self.NavigationIsValid`))
        (if (not _returnvalue)
          (set `self.CurrentCubeIndex` (- (`self.CurrentCubeIndex`) (`local.Direction`)))))
      (:`then_3`
        (`self.UpdateHighlightOfSelectedCube` true)))))

(fn `NavigationIsValid`
  (returns (ReturnValue :type Boolean))
  (bind _output (`self.GetSelectedColor`))
  (if (`|EnumEquality` (`self.CurrentColor`) "NewEnumerator0")
    (return true)
    (else
      ; Correct Keynode?
      (if (and (`/Game/Blueprints/ColorConnect/BP_ColorPuzzleComponent.IsKeyNode` _output) (`|EnumEquality` (`/Game/Blueprints/ColorConnect/BP_ColorPuzzleComponent.PuzzleColor` _output) (`self.CurrentColor`)) (!= _output (`self.SelectedKeyNode`)))
        (`self.ConnectKeyNodes`)
        (return true)
        (else
          ; Is Node with Empty Color?
          (if (`|EnumEquality` (`/Game/Blueprints/ColorConnect/BP_ColorPuzzleComponent.PuzzleColor` (`self.GetSelectedColor`)) "NewEnumerator0")
            (`/Game/Blueprints/ColorConnect/BP_ColorPuzzleComponent.ChangeColor` (`self.GetSelectedColor`) (`self.CurrentColor`))
            (return true)
            (else
              ; Must be colored Node
              (return false))))))))

(fn `Reset`
  (set `self.SelectedKeyNode` null)
  (for _array_element (`self.Cube`)
    (set `/Game/Blueprints/ColorConnect/BP_ColorPuzzleComponent.IsConnected` false _array_element)
    (if (not (`/Game/Blueprints/ColorConnect/BP_ColorPuzzleComponent.IsKeyNode` _array_element))
      (`/Game/Blueprints/ColorConnect/BP_ColorPuzzleComponent.ChangeColor` _array_element "NewEnumerator0")
      (set `self.CurrentColor` "NewEnumerator0"))))

(fn `SolvePuzzle`
  (`self.OnPuzzleSolved`)
  (set `self.CanBePossessed` false))

(fn `TrySelectNode`
  (bind _output (`self.GetSelectedColor`))
  (if (`/Game/Blueprints/ColorConnect/BP_ColorPuzzleComponent.IsKeyNode` _output)
    (if (not (`/Game/Blueprints/ColorConnect/BP_ColorPuzzleComponent.IsConnected` _output))
      (`KismetSystemLibrary.PrintString` "Selected")
      (set `self.SelectedKeyNode` _output)
      (set `self.CurrentColor` (`/Game/Blueprints/ColorConnect/BP_ColorPuzzleComponent.PuzzleColor` _output)))))

(fn `UpdateHighlightOfSelectedCube`
  (params (bEnable :type Boolean))
  (bind _output (`self.GetSelectedColor`))
  (if (`self.CanBePossessed`)
    (`self.SetHighlight` bEnable _output)
    (else
      (`self.SetHighlight` false _output))))

(fn `UserConstructionScript`
  (`parent.UserConstructionScript`))