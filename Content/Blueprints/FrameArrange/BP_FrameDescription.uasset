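; BP_FrameDescription is an interactable actor that shows descriptive dialogue text, apparently for a frame in the world.
; A box overlap toggles the visibility of its Widget component as something enters or leaves range.
; Interact plays a sound, creates a BPW_DialogUI on the player screen, fills it with the actor's text and character strings, and switches input to UI only with the mouse cursor shown.
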(event `/Game/Blueprints/InteractionInterface.Interact`
  (params (PlayerCharacter :type "/Game/Blueprints/Character/BP_FirstPersonCharacter Object Reference"))
  (bind _returnvalue (`GameplayStatics.GetPlayerController` 0))
  (bind _dialogui (`self.DialogUI`))
  (`GameplayStatics.PlaySound2D` "/Game/Audio/SFX/interact.interact" 1.0 1.0 0.0 null null)
  (`KismetSystemLibrary.PrintString` "Interacted")
  (bind _returnvalue_2 (`|CreateWidget` "/Game/UI/BPW/BPW_DialogUI.BPW_DialogUI_C" (`GameplayStatics.GetPlayerController` 0)))
  (bind _output_get (set `self.DialogUI` _returnvalue_2))
  (`UserWidget.AddToPlayerScreen` _output_get 0)
  (set `PlayerController.bShowMouseCursor` true _returnvalue)
  (`WidgetBlueprintLibrary.SetInputMode_UIOnlyEx` _returnvalue null)
  (set `TextBlock.Text` (`self.Text`) (`/Game/UI/BPW/BPW_DialogUI.TextBlock_Dialog` _dialogui))
  (set `TextBlock.Text` (`self.Chracter`) (`/Game/UI/BPW/BPW_DialogUI.TextBlock_Character` _dialogui)))

(event `self.Box.OnComponentBeginOverlap`
  (params (OverlappedComponent :type "PrimitiveComponent Object Reference") (OtherActor :type "Actor Object Reference") (OtherComp :type "PrimitiveComponent Object Reference") (OtherBodyIndex :type Integer) (bFromSweep :type Boolean) (SweepResult :type "HitResult Structure (by ref)"))
  (`SceneComponent.SetVisibility` (`self.Widget`) true false))

(event `self.Box.OnComponentEndOverlap`
  (params (OverlappedComponent :type "PrimitiveComponent Object Reference") (OtherActor :type "Actor Object Reference") (OtherComp :type "PrimitiveComponent Object Reference") (OtherBodyIndex :type Integer))
  (`SceneComponent.SetVisibility` (`self.Widget`) false false))

(fn `UserConstructionScript`)