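; BP_Gate is a double gate that swings open when its linked ColorConnect puzzle is solved.
; On BeginPlay it binds to the puzzle's OnPuzzleSolved event, which plays a 2D door sound and starts the OpenGate timeline.
; The timeline's alpha scales separate left and right angles to set the relative yaw of the two pivots.
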(event `self.ReceiveBeginPlay`
  (add `/Game/Blueprints/ColorConnect/BP_ColorConnect.OnPuzzleSolved` (`self.Color Connect`) (delegate `OnPuzzleSolved`)))

(event `OnPuzzleSolved`
  (`GameplayStatics.PlaySound2D` "/Game/Audio/SFX/GateDoorOpen.GateDoorOpen" 1.0 1.0 0.0 null null)
  (bind (_direction _open) (`Timeline|Open Gate`)
    (:`Update`
      (`SceneComponent.K2_SetRelativeRotation` (`self.LeftPivot`) (`KismetMathLibrary.MakeRotator` 0.0 0.0 (* _open (`self.AngleLeft`))) false false)
      (`SceneComponent.K2_SetRelativeRotation` (`self.RightPivot`) (`KismetMathLibrary.MakeRotator` 0.0 0.0 (* _open (`self.AngleRight`))) false false))))

(fn `UserConstructionScript`)