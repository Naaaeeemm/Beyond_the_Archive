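; BP_BarrierDoor is a two-panel sliding door that moves when its referenced ColorConnect puzzle is solved.
; On BeginPlay it binds SlideDoor to the puzzle's OnPuzzleSolved event, if that reference is valid.
; SlideDoor plays a timeline whose track scales the L and R values to set the relative X locations of Cube2 and Cube1 respectively.
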(event `self.ReceiveBeginPlay`
  (bind _color_connect (`self.Color Connect`))
  (`/Engine/EditorBlueprintResources/StandardMacros.IsValid` _color_connect
    (:`Is Valid`
      (add `/Game/Blueprints/ColorConnect/BP_ColorConnect.OnPuzzleSolved` _color_connect (delegate `Slide Door`)))))

(event `Slide Door`
  (bind (_direction _newtrack_0) (`Timeline|Timeline`)
    (:`Update`
      (`SceneComponent.K2_SetRelativeLocation` (`self.Cube2`) (`KismetMathLibrary.MakeVector` (* _newtrack_0 (`self.l`))) false false)
      (`SceneComponent.K2_SetRelativeLocation` (`self.Cube1`) (`KismetMathLibrary.MakeVector` (* _newtrack_0 (`self.r`))) false false))))

(fn `UserConstructionScript`)