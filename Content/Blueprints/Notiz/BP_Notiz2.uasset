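; BP_Notiz2 is an interactable note that shows lore text to the player on screen.
; Overlapping its sphere shows a widget component, and leaving hides it again.
; On Interact it creates a BPW_Notiz widget, adds it to the player screen, plays a paper sound and fills the date, header and three lore text blocks from its own variables.
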(event `/Game/Blueprints/InteractionInterface.Interact`
  (params (PlayerCharacter :type "/Game/Blueprints/Character/BP_FirstPersonCharacter Object Reference"))
  (bind _returnvalue (`|CreateWidget` "/Game/UI/BPW/BPW_Notiz.BPW_Notiz_C" (`GameplayStatics.GetPlayerController` 0)))
  (bind _output_get (set `self.NewVar` _returnvalue))
  (`UserWidget.AddToPlayerScreen` _output_get 0)
  (`GameplayStatics.PlaySound2D` "/Game/Audio/SFX/Paper.Paper" 1.0 1.0 0.0 null null)
  (set `TextBlock.Text` (`self.Date`) (`/Game/UI/BPW/BPW_Notiz.TextBlock_Date` (`self.NewVar`)))
  (set `TextBlock.Text` (`self.Header`) (`/Game/UI/BPW/BPW_Notiz.TextBlock_Header` (`self.NewVar`)))
  (set `TextBlock.Text` (`self.Text`) (`/Game/UI/BPW/BPW_Notiz.TextBlock_Lore_1` (`self.NewVar`)))
  (set `TextBlock.Text` (`self.Text 1`) (`/Game/UI/BPW/BPW_Notiz.TextBlock_Lore_2` (`self.NewVar`)))
  (set `TextBlock.Text` (`self.Text 2`) (`/Game/UI/BPW/BPW_Notiz.TextBlock_Lore_3` (`self.NewVar`))))

(event `self.Sphere.OnComponentBeginOverlap`
  (params (OverlappedComponent :type "PrimitiveComponent Object Reference") (OtherActor :type "Actor Object Reference") (OtherComp :type "PrimitiveComponent Object Reference") (OtherBodyIndex :type Integer) (bFromSweep :type Boolean) (SweepResult :type "HitResult Structure (by ref)"))
  (`SceneComponent.SetVisibility` (`self.Widget`) true false))

(event `self.Sphere.OnComponentEndOverlap`
  (params (OverlappedComponent :type "PrimitiveComponent Object Reference") (OtherActor :type "Actor Object Reference") (OtherComp :type "PrimitiveComponent Object Reference") (OtherBodyIndex :type Integer))
  (`SceneComponent.SetVisibility` (`self.Widget`) false false))

(fn `UserConstructionScript`)