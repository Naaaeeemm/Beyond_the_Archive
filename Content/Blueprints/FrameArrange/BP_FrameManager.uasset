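; BP_FrameManager watches a frame-arrangement puzzle and signals when all four frames are placed correctly.
; Every tick it polls IsSolved on its four referenced frames.
; Once all four report solved, a DoOnce gate prints a debug message and calls Call4FramesPlaced a single time.
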(event `self.ReceiveTick`
  (params (DeltaSeconds :type "Float (single-precision)"))
  (if (and (`/Game/Blueprints/FrameArrange/BP_FrameStand.IsSolved?` (`self.Frame`)) (`/Game/Blueprints/FrameArrange/BP_FrameStand.IsSolved?` (`self.Frame_0`)) (`/Game/Blueprints/FrameArrange/BP_FrameStand.IsSolved?` (`self.Frame_1`)) (`/Game/Blueprints/FrameArrange/BP_FrameStand.IsSolved?` (`self.Frame_2`)))
    (`/Engine/EditorBlueprintResources/StandardMacros.DoOnce` false
      (:`Completed`
        (`KismetSystemLibrary.PrintString` "all 4 placed right")
        (`self.4FramesPlaced`)))))

(fn `UserConstructionScript`)