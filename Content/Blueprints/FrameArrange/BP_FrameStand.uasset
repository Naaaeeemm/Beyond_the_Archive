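; Puzzle stand that accepts a carried frame and reports solved when it holds the wanted one.
; Interact checks that the player's held actor matches the accepted class and the stand is empty, then snaps it to the placement point and clears the player's hand.
; Placement compares the frame's number to WantedFrame and calls Solved on a match.
; Tick frees the stand once the frame is no longer attached to it.
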(event `FramePlaced`)

(event `FrameTakenBack`)

(event `/Game/Blueprints/InteractionInterface.Interact`
  (params (PlayerCharacter :type "/Game/Blueprints/Character/BP_FirstPersonCharacter Object Reference"))
  (bind _pickedupactor (`/Game/Blueprints/Character/BP_FirstPersonCharacter.PickedUpActor` PlayerCharacter))
  (`/Engine/EditorBlueprintResources/StandardMacros.IsValid` _pickedupactor
    (:`Is Valid`
      (if (== (`self.AcceptedPickupClass`) (`GameplayStatics.GetObjectClass` _pickedupactor))
        (`/Engine/EditorBlueprintResources/StandardMacros.IsValid` (`self.PlacedFrame`)
          (:`Is Not Valid`
            (`self.PlaceFrame` _pickedupactor)
            (set `/Game/Blueprints/Character/BP_FirstPersonCharacter.PickedUpActor` null PlayerCharacter)))))))

(event `self.ReceiveTick`
  (params (DeltaSeconds :type "Float (single-precision)"))
  (`self.NoFrame`))

(fn `NoFrame`
  (`/Engine/EditorBlueprintResources/StandardMacros.IsValid` (`self.PlacedFrame`)
    (:`Is Valid`
      (if (not (== (`self.GetAttachParentActor` (`self.PlacedFrame`)) self))
        (set `self.PlacedFrame` null)))))

(fn `PlaceFrame`
  (params (Frame :type "/Game/Blueprints/Pickups/BP_PickupActor Object Reference"))
  (bind _frame (`local.Frame`))
  (bind _output_get (set `self.PlacedFrame` Frame))
  (`self.K2_AttachToComponent` _output_get (`self.FramePlacement`) "None" "SnapToTarget" "SnapToTarget" "KeepWorld" true)
  (`/Game/Blueprints/Pickups/BP_PickupActor.GetPlaced` _frame)
  (bind _output_get_2 (set `/Game/Blueprints/Pickups/BP_PickupActor.FrameNumber` (`/Game/Blueprints/Pickups/BP_PickupActor.FrameNumber` _frame) _frame))
  (`self.RightFrame` _output_get_2))

(fn `RightFrame`
  (params (FrameNumber :type "/Game/Blueprints/Pickups/Enum/EFrameNumber Enum" :default "NewEnumerator0"))
  (if (`|EnumEquality` (`self.WantedFrame`) FrameNumber)
    (`KismetSystemLibrary.PrintString` "Right Frame")
    (`self.RightFrameSolved`)))

(fn `RightFrameSolved`
  (`self.Solved`))

(fn `UserConstructionScript`)