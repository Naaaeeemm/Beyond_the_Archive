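; BP_BookPlacement is an interactable slot in a book arrangement puzzle that accepts a carried book and checks whether it is the wanted one.
; Interact takes the player's held actor if its class matches and the slot is empty, then snaps it to the placement pivot.
; A matching book number calls Solved.
; Tick polls the book's attach parent to free the slot once the book is taken.
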(event `/Game/Blueprints/InteractionInterface.Interact`
  (params (PlayerCharacter :type "/Game/Blueprints/Character/BP_FirstPersonCharacter Object Reference"))
  (bind _pickedupactor (`/Game/Blueprints/Character/BP_FirstPersonCharacter.PickedUpActor` PlayerCharacter))
  (`/Engine/EditorBlueprintResources/StandardMacros.IsValid` _pickedupactor
    (:`Is Valid`
      (if (== (`self.AcceptedPickUpClass`) (`GameplayStatics.GetObjectClass` _pickedupactor))
        (`/Engine/EditorBlueprintResources/StandardMacros.IsValid` (`self.PlacedBook`)
          (:`Is Not Valid`
            (`self.PlaceBook` _pickedupactor)
            (set `/Game/Blueprints/Character/BP_FirstPersonCharacter.PickedUpActor` null PlayerCharacter)
            (set `/Game/Blueprints/Character/BP_FirstPersonCharacter.HasAnActor` false PlayerCharacter)))))))

(event `self.ReceiveTick`
  (params (DeltaSeconds :type "Float (single-precision)"))
  (`self.NoBook`))

(fn `IsRightBook?`
  (params (BookNumber :type "/Game/Blueprints/Pickups/Enum/EBookNumber Enum" :default "NewEnumerator0"))
  (returns (ReturnValue :type Boolean))
  (return (`|EnumEquality` (`self.WantedBook`) BookNumber)))

(fn `NoBook`
  (`/Engine/EditorBlueprintResources/StandardMacros.IsValid` (`self.PlacedBook`)
    (:`Is Valid`
      (if (not (== (`self.GetAttachParentActor` (`self.PlacedBook`)) self))
        (set `self.PlacedBook` null)
        (`KismetSystemLibrary.PrintString` "Book taken")))))

(fn `PlaceBook`
  (params (Book :type "/Game/Blueprints/Pickups/BP_PickupActor Object Reference"))
  (bind _book (`local.Book`))
  (bind _output_get (set `self.PlacedBook` Book))
  (`self.K2_AttachToComponent` _output_get (`self.PlacementPivot`) "None" "SnapToTarget" "SnapToTarget" "KeepWorld" true)
  (`/Game/Blueprints/Pickups/BP_PickupActor.GetPlaced` _book)
  (bind _output_get_2 (set `/Game/Blueprints/Pickups/BP_PickupActor.BookNumber` (`/Game/Blueprints/Pickups/BP_PickupActor.BookNumber` _book) _book))
  (if (`self.IsRightBook?` _output_get_2)
    (`KismetSystemLibrary.PrintString` "Right Book")
    (`self.RightBookSolved`)
    (else
      (`KismetSystemLibrary.PrintString` "Wrong Book"))))

(fn `RightBookSolved`
  (`self.Solved`))

(fn `UserConstructionScript`)