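; Player controller that owns Enhanced Input for the first-person character, handling walking and camera rotation.
; It adds the first-person mapping context on BeginPlay and caches the possessed pawn as BP_FirstPersonCharacter.
; Walk input is forwarded to the character's MoveInWorldDirection as a local X/Y direction, while camera input feeds its controller yaw and pitch.
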(event `self.ReceiveBeginPlay`
  ;[0.5677 0.5677 0.5677 0.5] Mapping Context
  (`EnhancedInputSubsystemInterface.AddMappingContext` (subsystem `EnhancedInputLocalPlayerSubsystem`) "/Game/Input/IMC_FirstPersonCharacter.IMC_FirstPersonCharacter" 0 (struct)))

(event `self.ReceivePossess`
  (params (PossessedPawn :type "Pawn Object Reference"))
  ;[0.875 0.3937 0.693 0.5] Posses
  (bind _asbp_first_person_character (cast `/Game/Blueprints/Character/BP_FirstPersonCharacter` PossessedPawn))
  (set `self.FirstPersonCharacter` _asbp_first_person_character))

(event `EnhancedInput|/Game/Input/Actions/IA_Walk`
  (params (ActionValue :type "Vector2D Structure") (ElapsedSeconds :type "Float (double-precision)") (TriggeredSeconds :type "Float (double-precision)") (InputAction :type "InputAction Object Reference" :default "/Game/Input/Actions/IA_Walk.IA_Walk"))
  ;[0.6615 0.6615 0.6615 0.5] Move
  (:`Triggered`
    (`/Game/Blueprints/Character/BP_FirstPersonCharacter.MoveInWorldDirection` (`self.FirstPersonCharacter`) (`KismetMathLibrary.MakeVector` ActionValue_X ActionValue_Y))))

(event `EnhancedInput|/Game/Input/Actions/IA_RotateCamera`
  (params (ActionValue :type "Vector2D Structure") (ElapsedSeconds :type "Float (double-precision)") (TriggeredSeconds :type "Float (double-precision)") (InputAction :type "InputAction Object Reference" :default "/Game/Input/Actions/IA_RotateCamera.IA_RotateCamera"))
  (bind _firstpersoncharacter (`self.FirstPersonCharacter`))
  ; RotateCamera
  (:`Triggered`
    (`Pawn.AddControllerYawInput` _firstpersoncharacter ActionValue_X)
    (`Pawn.AddControllerPitchInput` _firstpersoncharacter ActionValue_Y)))

(fn `UserConstructionScript`)