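; BP_BookManager is a puzzle manager that watches four book actors and reacts when all of them are solved.
; Each tick it checks IsSolved on Book1 through Book4.
; When all four report solved, a DoOnce gate prints a debug "Solved" message and fires CallAll4Solved a single time.
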(event `self.ReceiveTick`
  (params (DeltaSeconds :type "Float (single-precision)"))
  (if (and (`/Game/Blueprints/BookArrange/BP_BookPlacement.IsSolved?` (`self.Book1`) false) (`/Game/Blueprints/BookArrange/BP_BookPlacement.IsSolved?` (`self.Book2`) false) (`/Game/Blueprints/BookArrange/BP_BookPlacement.IsSolved?` (`self.Book3`) false) (`/Game/Blueprints/BookArrange/BP_BookPlacement.IsSolved?` (`self.Book4`) false))
    (`/Engine/EditorBlueprintResources/StandardMacros.DoOnce` false
      (:`Completed`
        (`KismetSystemLibrary.PrintString` "Solved")
        (`self.All4Solved`)))))

(fn `UserConstructionScript`)